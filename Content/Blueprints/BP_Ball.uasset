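; BP_Ball is a ball actor that reacts to entering a BP_Basket and plays impact audio.
; Overlapping a basket enables physics simulation and sets IsOverlapGoal, while other overlaps play BallHit from InitialVelocity if physics is off.
; Component hits within an impulse range also play BallHit, throttled by a DoOnce that resets after a short delay.
; Both sound paths map impact strength to volume and a pitch parameter.
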(event `self.ReceiveActorBeginOverlap`
  (params (OtherActor :type "Actor Object Reference"))
  (bind _ball (`self.Ball`))
  (bind _initialvelocity (`self.InitialVelocity`))
  (bind _ball_hit (`self.Ball_hit`))
  (cast `/Game/Basketball_template/Blueprints/BP_Basket` OtherActor
    (:`then`
      (`PrimitiveComponent.SetSimulatePhysics` _ball true)
      (set `self.isOverlapGoal` true))
    (:`CastFailed`
      (if (not (`SceneComponent.IsSimulatingPhysics` _ball "None"))
        (`AudioComponent.SetVolumeMultiplier` _ball_hit (`KismetMathLibrary.MapRangeClamped` _initialvelocity 0.0 10.0 0.0 1.0))
        (`AudioComponent.SetFloatParameter` _ball_hit "pitch" (`KismetMathLibrary.MapRangeClamped` _initialvelocity 2.0 10.0 0.85 1.2))
        (`AudioComponent.Play` _ball_hit 0.0)))))

(event `self.Ball.OnComponentHit`
  (params (HitComponent :type "PrimitiveComponent Object Reference") (OtherActor :type "Actor Object Reference") (OtherComp :type "PrimitiveComponent Object Reference") (NormalImpulse :type "Vector Structure") (Hit :type "HitResult Structure (by ref)"))
  (bind _returnvalue (`KismetMathLibrary.VSize` NormalImpulse))
  (bind _ball_hit (`self.Ball_hit`))
  (if (`KismetMathLibrary.InRange_FloatFloat` _returnvalue 50.0 30000.0)
    (`/Engine/EditorBlueprintResources/StandardMacros.DoOnce` false :!label _label
      (:`Completed`
        (`AudioComponent.SetVolumeMultiplier` _ball_hit (`KismetMathLibrary.MapRangeClamped` _returnvalue 0.0 3500.0 0.0 1.0))
        (`AudioComponent.SetFloatParameter` _ball_hit "pitch" (`KismetMathLibrary.MapRangeClamped` _returnvalue 20.0 1000.0 0.85 1.2))
        (`AudioComponent.Play` _ball_hit 0.0)
        (`KismetSystemLibrary.Delay` 0.2)
        (goto _label :!via `Reset`)))))

(fn `UserConstructionScript`)