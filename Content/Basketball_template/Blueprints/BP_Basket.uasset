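; BP_Basket is the basketball hoop actor, which tracks objects passing through it and plays impact audio.
; Ending overlap on Coll_1 increments Success, while ending overlap on Coll_2 plays a basketball cue.
; Cloth_collision overlaps store the overlapping component and a ClothOverlap flag.
; Basket hits within an impulse range play a ring sound with volume scaled by impulse, throttled by a DoOnce and short Delay.
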(event `self.Cloth_collision.OnComponentBeginOverlap`
  (params (OverlappedComponent :type "PrimitiveComponent Object Reference") (OtherActor :type "Actor Object Reference") (OtherComp :type "PrimitiveComponent Object Reference") (OtherBodyIndex :type Integer) (bFromSweep :type Boolean) (SweepResult :type "HitResult Structure (by ref)"))
  (set `self.component` OtherComp)
  (set `self.cloth_overlap` true))

(event `self.Cloth_collision.OnComponentEndOverlap`
  (params (OverlappedComponent :type "PrimitiveComponent Object Reference") (OtherActor :type "Actor Object Reference") (OtherComp :type "PrimitiveComponent Object Reference") (OtherBodyIndex :type Integer))
  (set `self.component` null)
  (set `self.cloth_overlap` false))

(event `self.coll_2.OnComponentEndOverlap`
  (params (OverlappedComponent :type "PrimitiveComponent Object Reference") (OtherActor :type "Actor Object Reference") (OtherComp :type "PrimitiveComponent Object Reference") (OtherBodyIndex :type Integer))
  (`AudioComponent.Play` (`self.basketball_red_Cue`) 0.0))

(event `self.coll_1.OnComponentEndOverlap`
  (params (OverlappedComponent :type "PrimitiveComponent Object Reference") (OtherActor :type "Actor Object Reference") (OtherComp :type "PrimitiveComponent Object Reference") (OtherBodyIndex :type Integer))
  (set `self.Success` (+ (`self.Success`) 1)))

(event `self.Basket.OnComponentHit`
  (params (HitComponent :type "PrimitiveComponent Object Reference") (OtherActor :type "Actor Object Reference") (OtherComp :type "PrimitiveComponent Object Reference") (NormalImpulse :type "Vector Structure") (Hit :type "HitResult Structure (by ref)"))
  (bind _returnvalue (`KismetMathLibrary.VSize` NormalImpulse))
  (bind _hit_ring_cue (`self.hit_ring_Cue`))
  (if (`KismetMathLibrary.InRange_FloatFloat` _returnvalue 20.0 10000.0)
    (`/Engine/EditorBlueprintResources/StandardMacros.DoOnce` false :!label _label
      (:`Completed`
        (`AudioComponent.SetVolumeMultiplier` _hit_ring_cue (`KismetMathLibrary.MapRangeClamped` _returnvalue 0.0 2000.0 0.0 1.0))
        (`AudioComponent.Play` _hit_ring_cue 0.0)
        (`KismetSystemLibrary.Delay` 0.2)
        (goto _label :!via `Reset`)))))

(fn `UserConstructionScript`)